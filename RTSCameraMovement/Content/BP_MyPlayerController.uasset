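; Player controller that drives a top-down style camera pawn with axis input and screen-edge panning, showing the mouse cursor on start.
; MoveForward and MoveRight shift the cached BP_MyCameraPawn along its local axes, with speed scaled by clamped spring arm length, so zoom affects pan rate.
; A screen-edge macro checks cursor position near viewport borders; MouseY updates forward speed, while only MouseX applies the local offset.
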(event `self.ReceiveBeginPlay`
  (`self.CastReferences`
    (:`ReturnNode`
      (set `self.bShowMouseCursor` true))))

(event `InputAxisKey|MouseX`
  (params (AxisValue :type "Float (single-precision)"))
  (bind (_deltaxspeed _deltayspeed) (`self.ScreenEdgeMovement` :!label _label)
    (:`ReturnNode`
      (`self.K2_AddActorLocalOffset` (`self.CameraPawnRef`) (`KismetMathLibrary.MakeVector` _deltaxspeed _deltayspeed) false false))))

(event `InputAxisKey|MouseY`
  (params (AxisValue :type "Float (single-precision)"))
  (goto _label :!via `MouseY`))

(event `InputAxis|MoveForward`
  (params (AxisValue :type "Float (single-precision)"))
  (bind _camerapawnref (`self.CameraPawnRef`))
  (`self.K2_SetActorTransform` _camerapawnref (`self.MovementX` AxisValue (`self.MovementSpeedCalculation`) (`self.MoveSensitivity`) _camerapawnref) false false))

(event `InputAxis|MoveRight`
  (params (AxisValue :type "Float (single-precision)"))
  (bind _camerapawnref (`self.CameraPawnRef`))
  (`self.K2_SetActorTransform` _camerapawnref (`self.MovementY` AxisValue (`self.MovementSpeedCalculation`) (`self.MoveSensitivity`) _camerapawnref) false false))

(fn `MovementSpeedCalculation`
  (returns (MoveSensitivity :type "Float (double-precision)"))
  (return (`KismetMathLibrary.FClamp` (/ (`SpringArmComponent.TargetArmLength` (`/Game/BP_MyCameraPawn.SpringArm` (`self.CameraPawnRef`))) 100.0) 5.0 20.0)))

(fn `UserConstructionScript`)